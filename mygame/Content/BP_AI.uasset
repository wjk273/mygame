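; BP_AI is a melee enemy character that chases and attacks the player once PawnSensing sees a pawn.
; AI MoveTo approaches the player, retrying on failure; on success it plays an attack montage, gated by CanAttack until completion or interruption.
; A montage notify sphere-traces forward and applies damage to the hit actor.
; Receiving any damage immediately ragdolls the mesh and disables movement, without a health check.
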(event OnSeePawn(PawnSensing)
  (params (Pawn :type Pawn%20Object%20Reference))
  (CallFunction|AIChasePlayer))

(event Custom|AI%20Chase%20Player
  (bind _returnvalue (Transformation|GetActorLocation))
  (AI|AIMoveTo self "0, 0, 0" (Game|GetPlayerCharacter 0) 1.2e+02 false
    (:OnSuccess
      (if (Variables|Default|GetcanAttack?)
        (Animation|Montage|PlayMontage (Variables|Character|GetMesh) "/Game/RamsterZ_FreeAnims_Volume1/AnimationSequence/H2H/attack_Montage.attack_Montage"
          (:then
            (Variables|Default|SetcanAttack? false))
          (:OnCompleted
            (Variables|Default|SetcanAttack? true :!label _label))
          (:OnInterrupted
            (goto _label))
          (:OnNotifyBegin
            (bind _outhit (Collision|SphereTraceByChannel _returnvalue (+ _returnvalue (* (Transformation|GetActorForwardVector) 8e+01)) 35.0 "TraceTypeQuery1" false 0 "ForDuration"))
            (if true
              (Game|Damage|ApplyDamage (.HitActor (Collision|BreakHitResult _outhit)) 1e+01 0 0))))))
    (:OnFail
      (CallFunction|AIChasePlayer))))

(event EventBeginPlay)

(event Game|Damage|EventAnyDamage
  (params (Damage :type Float%20%28single-precision%29) (DamageType :type Damage%20Type%20Object%20Reference) (InstigatedBy :type Controller%20Object%20Reference) (DamageCauser :type Actor%20Object%20Reference))
  (Physics|SetSimulatePhysics (Variables|Character|GetMesh) true)
  (Pawn|Components|CharacterMovement|DisableMovement (Variables|Character|GetCharacterMovement)))

(fn ConstructionScript)